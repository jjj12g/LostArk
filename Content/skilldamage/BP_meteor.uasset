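; BP_meteor is a meteor skill damage actor that applies a one-shot area hit, then removes itself.
; Shortly after BeginPlay, it gathers actors overlapping its Sphere and uses a dot product to keep only those in front of its forward vector.
; Those actors take fixed environmental damage with the meteor's owner as damage causer, and the actor destroys itself a few seconds later.
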(event `self.Sphere.OnComponentHit`
  (params (HitComponent :type "PrimitiveComponent Object Reference") (OtherActor :type "Actor Object Reference") (OtherComp :type "PrimitiveComponent Object Reference") (NormalImpulse :type "Vector Structure") (Hit :type "HitResult Structure (by ref)")))

(event `self.ReceiveBeginPlay`
  (`KismetSystemLibrary.Delay` 0.2)
  (for _array_element (`PrimitiveComponent.GetOverlappingActors` (`self.Sphere`) "/Script/Engine.Actor")
    (if (> (`KismetMathLibrary.Dot_VectorVector` (`KismetMathLibrary.GetDirectionUnitVector` (`self.K2_GetActorLocation`) (`self.K2_GetActorLocation` _array_element)) (`self.GetActorForwardVector`)) 0.0)
      (`GameplayStatics.ApplyDamage` _array_element 30.0 null (`self.GetOwner`) "/Engine/EngineDamageTypes/DmgTypeBP_Environmental.DmgTypeBP_Environmental_C")))
  (`KismetSystemLibrary.Delay` 3.0)
  (`self.K2_DestroyActor`))

(fn `UserConstructionScript`)