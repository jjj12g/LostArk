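; Attack component that provides two area attacks for its owner, a meteor-style magic circle and lightning.
; Each event spawns its effect actor with the given AttackTarget, sets the owning Pawn as instigator and binds to its AOE overlap callback.
; Overlapped actors receive the caller-supplied damage through a TakeDamage message, both attacks using the same damage type.
; The lightning event also runs straight into that damage call after binding.
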(event `metaor`
  (params (AttackTarget :type "Actor Object Reference") (Damage :type "Float (double-precision)"))
  (bind (_aspawn _bsuccess) (cast `Pawn` (`self.GetOwner`) :!pure true))
  (bind _returnvalue (`|SpawnActorFromClass` "/Game/AOE/BP_MagicCircle.BP_MagicCircle_C" (`KismetMathLibrary.MakeTransform` (0.0 0.0 0.0)) "Undefined" "MultiplyWithRoot" null AttackTarget true false false (select `bool` _bsuccess :`true` _aspawn)))
  (add `/Game/AOE/BP_AOE_Base.OnAOEOverlapActor` _returnvalue (delegate `DamagenemyAOE`)))

(event `DamagenemyAOE`
  (params (Actor :type "Actor Object Reference"))
  (message `/Game/BP_Attacks/Bpc_Attacks.TakeDamage` Actor (make `FallbackStruct` (stale `metaor` Damage) 0)))

(event `Lightning`
  (params (AttackTarget :type "Actor Object Reference") (Amount :type "Float (double-precision)"))
  (bind (_aspawn _bsuccess) (cast `Pawn` (`self.GetOwner`) :!pure true))
  (bind _returnvalue (`|SpawnActorFromClass` "/Game/AOE/BP_Lightning.BP_Lightning_C" (`KismetMathLibrary.MakeTransform` (0.0 0.0 0.0)) "Undefined" "MultiplyWithRoot" null AttackTarget true false false (select `bool` _bsuccess :`true` _aspawn)))
  (add `/Game/AOE/BP_AOE_Base.OnAOEOverlapActor` _returnvalue (delegate `lightdamage`))
  (message `/Game/BP_Attacks/Bpc_Attacks.TakeDamage` (stale `lightdamage` Actor) (make `FallbackStruct` Amount 0) :!label _label))

(event `lightdamage`
  (params (Actor :type "Actor Object Reference"))
  (goto _label))