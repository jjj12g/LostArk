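; Sorceress actor with a staff mesh, a minimap UI and a key-triggered Niagara effect.
; On BeginPlay it enables custom depth with a stencil value on the body and staff meshes, then creates the WB_Minimap widget and adds it to the viewport.
; Pressing Space Bar activates the Niagara component, then deactivates it after a short delay.
; An unconnected SpawnSystemAtLocation node never runs, and the construction script is empty.
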(event `self.ReceiveBeginPlay`
  (`PrimitiveComponent.SetCustomDepthStencilValue` (`self.Mesh`) 1)
  (`PrimitiveComponent.SetCustomDepthStencilValue` (`self.staffMeshComp`) 1)
  (`PrimitiveComponent.SetRenderCustomDepth` (`self.Mesh`) true)
  (`PrimitiveComponent.SetRenderCustomDepth` (`self.staffMeshComp`) true)
  (bind _returnvalue (`|CreateWidget` "/Game/mnimap/WB_Minimap.WB_Minimap_C" (`GameplayStatics.GetPlayerController` 0)))
  (`UserWidget.AddToViewport` _returnvalue 0))

(event `Key|SpaceBar`
  (params (Key :type "Key Structure"))
  (:`Pressed`
    (`ActorComponent.SetActive` (`self.Niagara`) true false)
    (`KismetSystemLibrary.Delay` 1.5)
    (`ActorComponent.SetActive` (`self.Niagara`) false false)))

(fn `UserConstructionScript`)