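; Top-down player character with a dash, melee slash, projectile, and meteor and lightning spells on input keys.
; The dash briefly boosts movement toward the controller's cached destination; slashes sphere-trace for pawns, projectiles report impacts back, and BpcAttacks casts spells at a found BP_enemy.
; Damage travels as SDamageInfo, with health delegated to BPCDamageSystem and shown in a widget.
; Custom depth marks the ally outline; death enables mesh physics.
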(event `Key|SpaceBar`
  (params (Key :type "Key Structure"))
  (bind _returnvalue (`GameplayStatics.GetPlayerController` 0))
  (bind _charactermovement (`self.CharacterMovement`))
  (bind _charactermovement_2 (`self.CharacterMovement`))
  (:`Pressed`
    (set `CharacterMovementComponent.MaxWalkSpeed` 1000.0 _charactermovement_2)
    (set `CharacterMovementComponent.MaxAcceleration` 90000.0 _charactermovement_2)
    (`Timeline|Timeline` :!via `PlayFromStart`
      (:`Update`
        (bind _asbp_top_down_controller (cast `/Game/TopDown/Blueprints/BP_TopDownController` _returnvalue))
        (`AIBlueprintHelperLibrary.SimpleMoveToLocation` _returnvalue (`/Game/TopDown/Blueprints/BP_TopDownController.CachedDestination` _asbp_top_down_controller)))
      (:`Finished`
        (set `CharacterMovementComponent.MaxWalkSpeed` 600.0 _charactermovement)
        (set `CharacterMovementComponent.MaxAcceleration` 1000.0 _charactermovement)))))

(event `self.ReceiveBeginPlay`
  (`|ExecutionSequence`
    (:`then_0`
      ;[1 1 1] 머리 위에 헬스바 Widget
      (bind _returnvalue (`|CreateWidget` "/Game/DamageSystem/W_HealthBar.W_HealthBar_C" null self))
      (`WidgetComponent.SetWidget` (`self.Widget`) _returnvalue)
      (`|CreateWidget` "/Game/DamageSystem/W_HealthBar.W_HealthBar_C" null null))
    (:`then_1`
      ;[1 1 1] Show the Player Mesh Outlines
      ; Value 1 = Ally
      (`PrimitiveComponent.SetCustomDepthStencilValue` (`self.Mesh`) 1)
      (`PrimitiveComponent.SetRenderCustomDepth` (`self.Mesh`) true))))

(event `Death`
  (bind _mesh (`self.Mesh`))
  (`KismetSystemLibrary.PrintString` "P Dead" true true (struct :`G` 0.658824 :`B` 1.0 :`A` 1.0) 50.0)
  (`PrimitiveComponent.SetSimulatePhysics` _mesh true)
  (`PrimitiveComponent.SetCollisionEnabled` _mesh "QueryAndPhysics"))

(event `Blocked`
  (params (CanBeParried :type Boolean))
  (`KismetSystemLibrary.PrintString` "P Blocked" true true (struct :`G` 0.658824 :`B` 1.0 :`A` 1.0) 50.0))

(event `DamageResponse`
  (params (DamageResponse :type "/Game/DamageSystem/E_DamageResponse Enum" :default "NewEnumerator0"))
  (`KismetSystemLibrary.PrintString` (`|GetEnumeratorNameAsString` DamageResponse) true true (struct :`G` 0.658824 :`B` 1.0 :`A` 1.0) 50.0)
  (switch `/Game/DamageSystem/E_DamageResponse` DamageResponse
    (:`NewEnumerator1`
      (`self.PlayAnimMontage` "/Game/Movement/Soccer_Trip_Montage.Soccer_Trip_Montage" 1.5))))

(event `Key|LeftMouseButton`
  (params (Key :type "Key Structure"))
  (bind _returnvalue (`self.K2_GetActorLocation`))
  (:`Pressed`
    (`self.PlayAnimMontage` "/Game/Movement/Sword_And_Shield_Slash_Montage.Sword_And_Shield_Slash_Montage" 1.5)
    ;[1 1 1] 스피어 트레이스 영역
    (bind (_outhit _returnvalue_2) (`KismetSystemLibrary.SphereTraceSingleForObjects` :`Start` _returnvalue :`End` (+ _returnvalue (* (`self.GetActorForwardVector`) 100.0)) :`Radius` 20.0 :`ObjectTypes` (`|MakeArray` "ObjectTypeQuery3" :!type "EObjectTypeQuery Enum") :`DrawDebugType` "ForDuration" :`DrawTime` 1.0))
    ;[1 1 1] 스피어 트레이스에 맞은 액터의 TakeDamage 함수 실행
    ; Amount : amount of health decrease
    (`KismetSystemLibrary.PrintString` "hit" true true (struct :`G` 0.658824 :`B` 1.0 :`A` 1.0) 50.0)
    (if _returnvalue_2
      (bind (_bblockinghit _binitialoverlap _time _distance _location _impactpoint _normal _impactnormal _physmat _hitactor) (`GameplayStatics.BreakHitResult` _outhit))
      (bind _wasdamaged (message `/Game/DamageSystem/BPI_Damagable.TakeDamage` _hitactor (make `/Game/DamageSystem/S_DamageInfo` 10.0 "NewEnumerator1" "NewEnumerator1")))
      (if _wasdamaged
        (`GameplayStatics.SpawnEmitterAtLocation` "/Game/StarterContent/Particles/P_Explosion.P_Explosion" _location)))))

(event `Key|E`
  (params (Key :type "Key Structure"))
  (:`Pressed`
    (`self.PlayAnimMontage` "/Game/Blueprints/Characters/AM_CharAttack.AM_CharAttack")
    (`KismetSystemLibrary.Delay` 0.5)
    (bind _returnvalue (`|SpawnActorFromClass` "/Game/projectiles/BP_projectile_Base.BP_projectile_Base_C" (`SceneComponent.K2_GetComponentToWorld` (`self.Scene`)) "Undefined" "MultiplyWithRoot" self 1000.0 0.0 null null))
    (add `/Game/projectiles/BP_projectile_Base.OnProjectileImpact` _returnvalue (delegate `Damage enemy`))
    (`PrimitiveComponent.IgnoreActorWhenMoving` (`self.CapsuleComponent`) _returnvalue true)))

(event `Damage enemy`
  (params (`other Actor` :type "Actor Object Reference") (Hit :type "HitResult Structure"))
  (message `/Game/DamageSystem/BPI_Damagable.TakeDamage` `other Actor` (make `/Game/DamageSystem/S_DamageInfo` 10.0 "NewEnumerator2" "NewEnumerator1")))

(event `Key|R`
  (params (Key :type "Key Structure"))
  (:`Pressed`
    (`self.PlayAnimMontage` "/Game/Movement/Sword_And_Shield_Slash_Montage.Sword_And_Shield_Slash_Montage")
    (bind _returnvalue (`GameplayStatics.GetActorOfClass` "/Game/Blueprints/Enemy/BP_Enemy.BP_enemy_C"))
    (`/Game/BP_Attacks/Bpc_Attacks.metaor` (`self.Bpc_Attacks`) _returnvalue 30.0)
    (`KismetSystemLibrary.Delay` 1.3)
    ;[1 1 1] PlayerController 의 카메라를 중심으로 카메라 흔들림
    (bind _asbp_player_top_down (cast `/Game/DamageSystem/Player/BP_PlayerTopDown` (`GameplayStatics.GetPlayerCharacter` 0)))
    (`GameplayStatics.PlayWorldCameraShake` "/Game/DamageSystem/CameraShake/BP_CameraShake.BP_CameraShake_C" (`SceneComponent.K2_GetComponentLocation` (`LostArkCharacter.TopDownCameraComponent` _asbp_player_top_down)) 0.0 500.0)))

(event `Key|W`
  (params (Key :type "Key Structure"))
  (:`Pressed`
    (`self.PlayAnimMontage` "/Game/Movement/Sword_And_Shield_Slash_Montage.Sword_And_Shield_Slash_Montage")
    (bind _returnvalue (`GameplayStatics.GetActorOfClass` "/Game/Blueprints/Enemy/BP_Enemy.BP_enemy_C"))
    (`/Game/BP_Attacks/Bpc_Attacks.Lightning` (`self.Bpc_Attacks`) _returnvalue 20.0)
    (`KismetSystemLibrary.Delay` 0.0)
    ;[1 1 1] PlayerController 의 카메라를 중심으로 카메라 흔들림
    (bind _asbp_player_top_down (cast `/Game/DamageSystem/Player/BP_PlayerTopDown` (`GameplayStatics.GetPlayerCharacter` 0)))
    (`GameplayStatics.PlayWorldCameraShake` "/Game/DamageSystem/CameraShake/BP_CameraShake.BP_CameraShake_C" (`SceneComponent.K2_GetComponentLocation` (`LostArkCharacter.TopDownCameraComponent` _asbp_player_top_down)) 0.0 500.0)))

(fn `GetCurrentHealth`
  (returns (Health :type "Float (double-precision)"))
  (return (`/Game/DamageSystem/BPC_DamageSystem.Health` (`self.BPC_DamageSystem`))))

(fn `GetMaxHealth`
  (returns (MaxHealth :type "Float (double-precision)"))
  (return (`/Game/DamageSystem/BPC_DamageSystem.MaxHealth` (`self.BPC_DamageSystem`))))

(fn `Heal`
  (params (Amount :type "Float (double-precision)"))
  (returns (NewHealth :type "Float (double-precision)"))
  (bind _newhealth (`/Game/DamageSystem/BPC_DamageSystem.Heal` (`self.BPC_DamageSystem`) Amount))
  (return _newhealth))

(fn `TakeDamage`
  (params (DamageInfo :type "/Game/DamageSystem/S_DamageInfo Structure"))
  (returns (WasDamaged :type Boolean))
  (bind _wasdamaged (`/Game/DamageSystem/BPC_DamageSystem.TakeDamage` (`self.BPC_DamageSystem`) DamageInfo))
  (return _wasdamaged))

(fn `UserConstructionScript`)