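; Base projectile Blueprint with configurable speed, gravity, target and optional homing, driven by a ProjectileMovement component.
; The construction script applies those settings and, when homing, tracks the target's root component.
; On BeginPlay it ignores its owner when moving and aims its velocity at any valid target.
; On a box collision hit it calls OnProjectileImpact, spawns an impact effect and sound, then destroys itself.
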(event `self.ReceiveBeginPlay`
  (`PrimitiveComponent.IgnoreActorWhenMoving` (`self.BoxCollsion`) (`self.GetOwner`) true)
  (`self.Targrt`
    (:`then`
      (`self.RotateTOTarget`))
    (:`else`)))

(event `RotateTOTarget`
  (set `MovementComponent.Velocity` (* (`KismetMathLibrary.GetDirectionUnitVector` (`self.K2_GetActorLocation`) (`self.K2_GetActorLocation` (`self.Targrt`))) (`self.Speed`)) (`self.ProjectileMovement`)))

(event `self.BoxCollsion.OnComponentHit`
  (params (HitComponent :type "PrimitiveComponent Object Reference") (OtherActor :type "Actor Object Reference") (OtherComp :type "PrimitiveComponent Object Reference") (NormalImpulse :type "Vector Structure") (Hit :type "HitResult Structure (by ref)"))
  (bind (_bblockinghit _binitialoverlap _time _distance _location) (`GameplayStatics.BreakHitResult` Hit))
  (`self.OnProjectileImpact` OtherActor Hit)
  (`NiagaraFunctionLibrary.SpawnSystemAtLocation` (`self.impactEffect`) _location)
  (`GameplayStatics.PlaySoundAtLocation` (`self.Sound`) _location (struct) 1.0 1.0 0.0 null null null null)
  (`self.K2_DestroyActor`))

(fn `UserConstructionScript`
  (bind _projectilemovement (`self.ProjectileMovement`))
  (set `ProjectileMovementComponent.InitialSpeed` (`self.Speed`) _projectilemovement)
  (set `ProjectileMovementComponent.MaxSpeed` (`self.Speed`) _projectilemovement)
  (set `ProjectileMovementComponent.ProjectileGravityScale` (`self.Gravity`) _projectilemovement)
  (`self.Targrt`
    (:`then`
      (if (`self.isHoming`)
        (set `ProjectileMovementComponent.bIsHomingProjectile` true _projectilemovement)
        (set `ProjectileMovementComponent.HomingTargetComponent` (`Actor.RootComponent` (`self.Targrt`)) _projectilemovement)))
    (:`else`)))