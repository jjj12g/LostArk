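; Enemy actor that periodically attacks while alive, shows a health bar widget and can be damaged or healed.
; A looping timer runs a forward sphere trace against pawns, sending damage through interface messages and spawning an explosion when damage lands.
; Its damage interface functions delegate to BPCDamageSystem, whose bound events drive hit-reaction montages, a debug print on block, and physics-simulated death followed by delayed destruction.
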(event `self.ReceiveBeginPlay`
  (`KismetSystemLibrary.K2_SetTimerDelegate` (delegate `Attack`) 2.0 true) ; Every 2 seconds,\nrun Attack Event
  ;[1 1 1] 액터 위에 헬스바 위젯 표시
  (bind _returnvalue (`|CreateWidget` "/Game/DamageSystem/W_HealthBar.W_HealthBar_C" null self))
  (`WidgetComponent.SetWidget` (`self.Widget`) _returnvalue))

(event `Attack`
  (bind _returnvalue (`self.K2_GetActorLocation`))
  (if (not (`/Game/DamageSystem/BPC_DamageSystem.IsDead` (`self.BPC_DamageSystem`)))
    ;[1 1 1] 공격 콜리젼 = Sphere Trace
    ; 스피어 트레이스 영역 setting
    (bind (_outhit _returnvalue_2) (`KismetSystemLibrary.SphereTraceSingleForObjects` :`Start` _returnvalue :`End` (+ _returnvalue (* (`self.GetActorForwardVector`) 100.0)) :`Radius` 20.0 :`ObjectTypes` (`|MakeArray` "ObjectTypeQuery3" :!type "EObjectTypeQuery Enum") :`DrawDebugType` "ForDuration" :`TraceColor` (struct :`R` 0.027183 :`B` 1.0 :`A` 1.0) :`TraceHitColor` (struct :`R` 0.84175 :`B` 1.0 :`A` 1.0) :`DrawTime` 1.0))
    ;[1 1 1] 공격에 닿은 액터의 TakeDamage 함수 실행
    ; Amount : amount of decreased health
    (`KismetSystemLibrary.PrintString` "hit" true true (struct :`G` 0.658824 :`B` 1.0 :`A` 1.0) 50.0)
    (if _returnvalue_2
      (bind (_bblockinghit _binitialoverlap _time _distance _location _impactpoint _normal _impactnormal _physmat _hitactor) (`GameplayStatics.BreakHitResult` _outhit))
      (bind _wasdamaged (message `/Game/DamageSystem/BPI_Damagable.TakeDamage` _hitactor (make `/Game/DamageSystem/S_DamageInfo` 10.0 "NewEnumerator1" "NewEnumerator1")))
      (if _wasdamaged
        (`GameplayStatics.SpawnEmitterAtLocation` "/Game/StarterContent/Particles/P_Explosion.P_Explosion" _location)))))

(event `Death`
  (bind _mesh (`self.Mesh`))
  (`KismetSystemLibrary.PrintString` "E Dead" true true (struct :`R` 0.5 :`B` 1.0 :`A` 1.0) 50.0)
  (`PrimitiveComponent.SetSimulatePhysics` _mesh true)
  (`PrimitiveComponent.SetCollisionEnabled` _mesh "QueryAndPhysics")
  (`KismetSystemLibrary.Delay` 7.0)
  (`self.K2_DestroyActor`))

(event `Blocked`
  (params (CanBeParried :type Boolean))
  (`KismetSystemLibrary.PrintString` "E Blocked" true true (struct :`R` 0.501961 :`B` 1.0 :`A` 1.0) 50.0))

(event `DamageResponse`
  (params (DamageResponse :type "/Game/DamageSystem/E_DamageResponse Enum" :default "NewEnumerator0"))
  (switch `/Game/DamageSystem/E_DamageResponse` DamageResponse ; CAN JUSTIFY DIFFERENT RESPONSES\nTO EVERY OTHER DAMAGE TYPES
    (:`NewEnumerator1`
      (`|PlayMontage` null))))

(fn `GetCurrentHealth`
  (returns (Health :type "Float (double-precision)"))
  (return (`/Game/DamageSystem/BPC_DamageSystem.Health` (`self.BPC_DamageSystem`))))

(fn `GetMaxHealth`
  (returns (MaxHealth :type "Float (double-precision)"))
  (return (`/Game/DamageSystem/BPC_DamageSystem.MaxHealth` (`self.BPC_DamageSystem`))))

(fn `Heal`
  (params (Amount :type "Float (double-precision)"))
  (returns (NewHealth :type "Float (double-precision)"))
  (bind _newhealth (`/Game/DamageSystem/BPC_DamageSystem.Heal` (`self.BPC_DamageSystem`) Amount))
  (return _newhealth))

(fn `TakeDamage`
  (params (DamageInfo :type "/Game/DamageSystem/S_DamageInfo Structure"))
  (returns (WasDamaged :type Boolean))
  (bind _wasdamaged (`/Game/DamageSystem/BPC_DamageSystem.TakeDamage` (`self.BPC_DamageSystem`) DamageInfo))
  (return _wasdamaged))

(fn `UserConstructionScript`
  (bind _bpc_damagesystem (`self.BPC_DamageSystem`))
  (add `/Game/DamageSystem/BPC_DamageSystem.OnDeath` _bpc_damagesystem (`|CreateDelegate` :!event `Death`))
  (add `/Game/DamageSystem/BPC_DamageSystem.OnBlocked` _bpc_damagesystem (`|CreateDelegate` :!event `Blocked`))
  (add `/Game/DamageSystem/BPC_DamageSystem.OnDamageResponse` _bpc_damagesystem (`|CreateDelegate` :!event `DamageResponse`))
  (bind _health (message `/Game/DamageSystem/BPI_Damagable.GetCurrentHealth` self))
  (`KismetSystemLibrary.PrintString` (`KismetStringLibrary.Conv_DoubleToString` _health) true true (struct :`R` 0.501961 :`B` 1.0 :`A` 1.0)))