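; BP_SlashChar is a top-down character with a Space Bar dash toward the player controller's cached destination.
; The dash sharply raises walk speed and acceleration, reissues Simple Move To Location on each timeline update, and restores lower movement values on finish.
; Health getters, Heal and TakeDamage are thin wrappers that forward to the BPCDamageSystem component.
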(event `Key|SpaceBar`
  (params (Key :type "Key Structure"))
  (bind _returnvalue (`GameplayStatics.GetPlayerController` 0))
  (bind _charactermovement (`self.CharacterMovement`))
  (bind _charactermovement_2 (`self.CharacterMovement`))
  (:`Pressed`
    (set `CharacterMovementComponent.MaxWalkSpeed` 1000.0 _charactermovement_2)
    (set `CharacterMovementComponent.MaxAcceleration` 90000.0 _charactermovement_2)
    (`Timeline|Timeline` :!via `PlayFromStart`
      (:`Update`
        (bind _asbp_top_down_controller (cast `/Game/TopDown/Blueprints/BP_TopDownController` _returnvalue))
        (`AIBlueprintHelperLibrary.SimpleMoveToLocation` _returnvalue (`/Game/TopDown/Blueprints/BP_TopDownController.CachedDestination` _asbp_top_down_controller)))
      (:`Finished`
        (set `CharacterMovementComponent.MaxWalkSpeed` 600.0 _charactermovement)
        (set `CharacterMovementComponent.MaxAcceleration` 1000.0 _charactermovement)))))

(fn `GetCurrentHealth`
  (returns (Health :type "Float (double-precision)"))
  (return (`/Game/DamageSystem/BPC_DamageSystem.Health` (`self.BPC_DamageSystem`))))

(fn `GetMaxHealth`
  (returns (MaxHealth :type "Float (double-precision)"))
  (return (`/Game/DamageSystem/BPC_DamageSystem.MaxHealth` (`self.BPC_DamageSystem`))))

(fn `Heal`
  (params (Amount :type "Float (double-precision)"))
  (returns (NewHealth :type "Float (double-precision)"))
  (bind _newhealth (`/Game/DamageSystem/BPC_DamageSystem.Heal` (`self.BPC_DamageSystem`) Amount))
  (return _newhealth))

(fn `TakeDamage`
  (params (DamageInfo :type "/Game/DamageSystem/S_DamageInfo Structure"))
  (returns (WasDamaged :type Boolean))
  (bind _wasdamaged (`/Game/DamageSystem/BPC_DamageSystem.TakeDamage` (`self.BPC_DamageSystem`) DamageInfo))
  (return _wasdamaged))

(fn `UserConstructionScript`)