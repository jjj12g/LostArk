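; BP_WOLF is a wolf AI pawn that chases the player once its PawnSensing component sees a pawn.
; Any sighting, with no check on which pawn it is, sets a seeing flag that is never cleared and calls followplayer, which issues AI MoveTo toward player character 0.
; Random roaming and jump-bite animation logic are left disconnected, and the box overlap event is empty.
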(event `self.ReceiveBeginPlay`)

(event `self.Box.OnComponentBeginOverlap`
  (params (OverlappedComponent :type "PrimitiveComponent Object Reference") (OtherActor :type "Actor Object Reference") (OtherComp :type "PrimitiveComponent Object Reference") (OtherBodyIndex :type Integer) (bFromSweep :type Boolean) (SweepResult :type "HitResult Structure (by ref)")))

(event `Roam Around`)

(event `self.PawnSensing.OnSeePawn`
  (params (Pawn :type "Pawn Object Reference"))
  (set `self.isseeingplayer` true)
  (`self.follow player`))

(event `follow player`
  (if (`self.isseeingplayer`)
    (`|AIMoveTo` self (0.0 0.0 0.0) (`GameplayStatics.GetPlayerCharacter` 0))))

(fn `UserConstructionScript`)