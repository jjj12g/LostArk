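; BP_SlashChar is a player character Blueprint that marks its mesh as an ally for outline rendering.
; On BeginPlay it enables custom depth and sets the ally stencil value, its only live logic.
; Disconnected leftovers sketch meteor and lightning attacks through BpcAttacks, a projectile spawn, and a timeline dash toward the top-down controller's cached destination.
; The Damageenemy event and construction script are empty.
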(event `self.ReceiveBeginPlay`
  ;[1 1 1] Show the Player Mesh Outlines
  ; Value 1 = Ally
  (`PrimitiveComponent.SetCustomDepthStencilValue` (`self.Mesh`) 1)
  (`PrimitiveComponent.SetRenderCustomDepth` (`self.Mesh`) true))

(event `Key|SpaceBar`
  (params (Key :type "Key Structure")))

(event `Key|E`
  (params (Key :type "Key Structure")))

(event `Damage enemy`
  (params (`other Actor` :type "Actor Object Reference") (Hit :type "HitResult Structure")))

(event `Key|R`
  (params (Key :type "Key Structure")))

(event `Key|W`
  (params (Key :type "Key Structure")))

(fn `UserConstructionScript`)